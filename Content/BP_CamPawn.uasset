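; BP_CamPawn is a camera pawn that drives the car HUD for the car it is currently viewing.
; On BeginPlay it creates a WBP_CarHUD widget for the first player controller and adds it to the viewport.
; Each tick it takes the current car, casts its controller to AICarController, and copies the completed lap count into the HUD.
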(event `self.ReceiveBeginPlay`
  (bind _returnvalue (`|CreateWidget` "/Game/WBP_CarHUD.WBP_CarHUD_C" (`GameplayStatics.GetPlayerController` 0)))
  (set `self.HUD` _returnvalue)
  (`UserWidget.AddToViewport` _returnvalue 0))

(event `self.ReceiveActorBeginOverlap`
  (params (OtherActor :type "Actor Object Reference")))

(event `self.ReceiveTick`
  (params (DeltaSeconds :type "Float (single-precision)"))
  (bind _returnvalue (`self.GetCurrentCar`))
  (bind _ascar_pawn (cast `CarPawn` _returnvalue))
  (bind _asaicar_controller (cast `AICarController` (`self.GetController` _ascar_pawn)))
  (bind _returnvalue_2 (`AICarController.GetLapsCompleted` _asaicar_controller))
  (set `/Game/WBP_CarHUD.LapsCompleted` _returnvalue_2 (`self.HUD`)))

(fn `UserConstructionScript`)